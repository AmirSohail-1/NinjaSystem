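; BP_TestCharacter is a test character Blueprint that activates its Camera on BeginPlay.
; It also holds disconnected quest test logic that never runs: a delayed start, print and completion of QuestName.
; A second unwired chain creates a WBP_QuestWidgetShow, updates its quest list and adds it to the viewport.
; Tick, overlap and the construction script do nothing.
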(event `self.ReceiveBeginPlay`
  (`|ExecutionSequence`
    (:`then_0`
      ;[1 1 1] Comment
      (`ActorComponent.SetActive` (`self.Camera`) true false))))

(fn `UserConstructionScript`)